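; BP_TableLight is a spotlight for the pinball table that switches off when the game resets.
; On BeginPlay it binds to the pinball game mode's OnGameReset event, whose handler sets the spotlight intensity to zero without updating the on/off flag.
; A LoopLight event toggles that flag and the intensity, but the looping timer meant to call it is disconnected.
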(event Custom|LoopLight
  (bind _spotlight (Variables|Default|GetSpotLight))
  (if (Variables|Default|GetIsSpotLightOn?)
    (Variables|Default|SetIsSpotLightOn? false)
    (Rendering|Components|Light|SetIntensity _spotlight 0.0)
    (else
      (Variables|Default|SetIsSpotLightOn? true)
      (Rendering|Components|Light|SetIntensity _spotlight 1e+06))))

(event Custom|ResetTableLight
  (Rendering|Components|Light|SetIntensity (Variables|Default|GetSpotLight) 0.0))

(event EventBeginPlay
  (bind _asbp_pinball_game_mode (Utilities|Casting|CastToBP_PinballGameMode (Game|GetGameMode)))
  (EventDispatchers|BindEventtoOnGameReset _asbp_pinball_game_mode (delegate Custom|ResetTableLight)))

(fn ConstructionScript)