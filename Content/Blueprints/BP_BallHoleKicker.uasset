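; Pinball kicker hole that captures an overlapping BP_Ball, awards points and ejects it after a short delay.
; On overlap it zeroes the ball's speed, plays a sound, adds score through BP_PinballGameMode and sinks the ball below the hole's origin.
; After the delay it restores speed, nudges the ball up and along world Y, then plays a kickout sound and spark effect.
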(event Collision|EventActorBeginOverlap
  (params (OtherActor :type Actor%20Object%20Reference))
  (bind _self self)
  (bind _ballholemesh (Variables|Default|GetBallHoleMesh))
  (bind _returnvalue (Transformation|GetWorldLocation _ballholemesh))
  (bind _returnvalue_2 (Transformation|GetActorLocation _self))
  (Development|PrintString "Ball Hit Switch" false false)
  (bind _asbp_ball (Utilities|Casting|CastToBP_Ball OtherActor))
  (Default|AdjustBallSpeed _asbp_ball 0.0)
  (Audio|SpawnSoundAttached "/Game/Assets/Sounds/Pinball/Arcade_GameStart.Arcade_GameStart" (Variables|Default|GetBallHoleMesh) "None" "0, 0, 0" "0, 0, 0" "KeepRelativeOffset" false 1.0 1.0 0.0 0 0)
  (Development|PrintString "Kicker Hole" false false)
  (CallFunction|AddtoScore 5e+02)
  (Transformation|SetActorLocation _asbp_ball (Math|Vector|MakeVector (.x _returnvalue_2) (.y _returnvalue_2) (- (.z _returnvalue_2) 5e+01)) false false)
  (Utilities|FlowControl|Delay 1.0)
  (Default|AdjustBallSpeed _asbp_ball 2e+03)
  (Transformation|SetActorLocation _asbp_ball (Math|Vector|MakeVector (.x (Transformation|GetActorLocation _asbp_ball)) (+ (.y (Transformation|GetActorLocation _asbp_ball)) 5e+01) (+ (.z (Transformation|GetActorLocation _asbp_ball)) 6e+01)) false false)
  (Audio|SpawnSoundAttached "/Game/Assets/Sounds/Pinball/Pinball_BallKickout.Pinball_BallKickout" (Variables|Default|GetBallHoleMesh) "None" "0, 0, 0" "0, 0, 0" "KeepRelativeOffset" false 1.0 1.0 0.0 0 0)
  (Effects|SpawnEmitteratLocation "/Game/Assets/Particles/P_BumperSparks.P_BumperSparks" (Math|Vector|MakeVector (.x _returnvalue) (.y _returnvalue) (+ (.z _returnvalue) 5e+01))))

(fn ConstructionScript)

(fn AddtoScore
  (params (PointsToAdd :type Float%20%28single-precision%29))
  (bind _asbp_pinball_game_mode (Utilities|Casting|CastToBP_PinballGameMode (Game|GetGameMode)))
  (Default|AddScore _asbp_pinball_game_mode PointsToAdd))