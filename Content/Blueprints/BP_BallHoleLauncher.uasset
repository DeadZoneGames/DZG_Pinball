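; Pinball hole that captures a ball and lets the player aim and fire it back out.
; On overlap it stops the ball, awards points, sinks it briefly, moves it to the launch point with effects and blends the view to itself.
; Timelines swing the Launcher left or right.
; StopCharge restores ball speed, animates the plunger and returns the view to the first CameraActor found; ChargeLauncher is empty.
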(event Custom|ChargeLauncher
  (if (Variables|Default|GetBallInLauncher?)
    _))

(event Custom|StopCharge
  (bind _bp_ballref (Variables|Default|GetBP_BallRef))
  (if (Variables|Default|GetBallInLauncher?)
    (Development|PrintString "Stop Charge - Ball in Launcher" false false)
    (Utilities|IsValid _bp_ballref
      (:Is%20Valid
        (Default|AdjustBallSpeed _bp_ballref 2e+03))
      (:Is%20Not%20Valid
        _))
    (Components|MoveComponentTo (Variables|Default|GetLauncherPlunger) "0,-115.000000, 0" "0, 0,-90.000000" false false 0.04 false)
    (Components|MoveComponentTo (Variables|Default|GetLauncherPlunger) "0,115.000000, 0" "0, 0,-90.000000" false false 0.04 false)
    (bind _outactors (Actor|GetAllActorsOfClass "/Script/Engine.CameraActor"))
    (Game|Player|SetViewTargetwithBlend (Game|GetPlayerController 0) (Utilities|Array|Get(acopy) _outactors) 0.25 "VTBlend_Linear" 2.0 false)))

(event Custom|RotateLeft
  (bind _aimingalpha (Timeline|LeftAimingTimeline PlayFromStart)
    (:Update
      (Transformation|SetRelativeRotation (Variables|Default|GetLauncher) (Math|Rotator|Lerp(Rotator) (Variables|/Script/Engine.SceneComponent|GetRelativeRotation (Variables|Default|GetLauncher)) "0,-135.000000, 0" _aimingalpha) false false))))

(event Custom|RotateRight
  (bind _aimingalpha (Timeline|RightAimingTimeline PlayFromStart)
    (:Update
      (Transformation|SetRelativeRotation (Variables|Default|GetLauncher) (Math|Rotator|Lerp(Rotator) (Variables|/Script/Engine.SceneComponent|GetRelativeRotation (Variables|Default|GetLauncher)) "0,135.000000, 0" _aimingalpha) false false))))

(event Custom|StopRotation
  (Utilities|FlowControl|Sequence
    (:then_0
      (bind _aimingalpha (Timeline|LeftAimingTimeline Stop)
        (:Update
          (Transformation|SetRelativeRotation (Variables|Default|GetLauncher) (Math|Rotator|Lerp(Rotator) (Variables|/Script/Engine.SceneComponent|GetRelativeRotation (Variables|Default|GetLauncher)) "0,-135.000000, 0" _aimingalpha) false false))))
    (:then_1
      (bind _aimingalpha_2 (Timeline|RightAimingTimeline Stop)
        (:Update
          (Transformation|SetRelativeRotation (Variables|Default|GetLauncher) (Math|Rotator|Lerp(Rotator) (Variables|/Script/Engine.SceneComponent|GetRelativeRotation (Variables|Default|GetLauncher)) "0,135.000000, 0" _aimingalpha_2) false false))))))

(event Custom|ResetLauncher
  (bind _launcher (Variables|Default|GetLauncher))
  (Components|MoveComponentTo _launcher (Variables|/Script/Engine.SceneComponent|GetRelativeLocation _launcher) "0, 0, 0" false false 0.2 false))

(event EventBeginPlay
  (bind _asbp_pinball_game_mode (Utilities|Casting|CastToBP_PinballGameMode (Game|GetGameMode)))
  (EventDispatchers|BindEventtoOnGameReset _asbp_pinball_game_mode (EventDispatchers|CreateEvent :!event Custom|ResetLauncher)))

(event Collision|EventActorBeginOverlap
  (params (OtherActor :type Actor%20Object%20Reference))
  (bind _self self)
  (bind _ballholemesh (Variables|Default|GetBallHoleMesh))
  (bind _returnvalue (Transformation|GetWorldLocation _ballholemesh))
  (bind _returnvalue_2 (Transformation|GetActorLocation _self))
  (Development|PrintString "Ball Hit Switch" false false)
  (bind _asbp_ball (Utilities|Casting|CastToBP_Ball OtherActor))
  (Variables|Default|SetBP_BallRef _asbp_ball)
  (Variables|Default|SetBallInLauncher? true)
  (Default|AdjustBallSpeed (Variables|Default|GetBP_BallRef) 0.0)
  (Audio|SpawnSoundAttached "/Game/Assets/Sounds/Pinball/Arcade_GameStart.Arcade_GameStart" (Variables|Default|GetBallHoleMesh) "None" "0, 0, 0" "0, 0, 0" "KeepRelativeOffset" false 1.0 1.0 0.0 0 0)
  (Development|PrintString "Launcher Hole" false false)
  (CallFunction|AddtoScore 5e+02)
  (Transformation|SetActorLocation (Variables|Default|GetBP_BallRef) (Math|Vector|MakeVector (.x _returnvalue_2) (.y _returnvalue_2) (- (.z _returnvalue_2) 5e+01)) false false)
  (Utilities|FlowControl|Delay 1.0)
  (Transformation|SetActorLocation (Variables|Default|GetBP_BallRef) (CallFunction|GetBallLaunchLocation) false false)
  (Audio|SpawnSoundAttached "/Game/Assets/Sounds/Pinball/Pinball_BallKickout.Pinball_BallKickout" (Variables|Default|GetBallHoleMesh) "None" "0, 0, 0" "0, 0, 0" "KeepRelativeOffset" false 1.0 1.0 0.0 0 0)
  (Effects|SpawnEmitteratLocation "/Game/Assets/Particles/P_BumperSparks.P_BumperSparks" (Math|Vector|MakeVector (.x _returnvalue) (.y _returnvalue) (+ (.z _returnvalue) 5e+01)))
  (Game|Player|SetViewTargetwithBlend (Game|GetPlayerController 0) self 1.0 "VTBlend_Linear" 0.0 false))

(fn ConstructionScript)

(fn AddtoScore
  (params (PointsToAdd :type Float%20%28single-precision%29))
  (bind _asbp_pinball_game_mode (Utilities|Casting|CastToBP_PinballGameMode (Game|GetGameMode)))
  (Default|AddScore _asbp_pinball_game_mode PointsToAdd))

(fn GetBallLaunchLocation
  (return (Math|Transform|TransformLocation (Transformation|GetActorTransform) (Variables|Default|GetBallLaunchLocation))))