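; Black hole target in a pinball game that swallows any ball overlapping it, awards points and respawns a ball elsewhere.
; On overlap it stops the ball, plays a sound, adds score through BP_PinballGameMode and sinks the ball below the hole.
; After a short delay, a warp sound and timeline shrink the ball to nothing, then destroy it and have the game mode spawn one at a random kicker hole.
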(event Collision|EventActorBeginOverlap
  (params (OtherActor :type Actor%20Object%20Reference))
  (bind _self self)
  (bind _returnvalue (Transformation|GetActorLocation _self))
  (Development|PrintString "Ball Hit Switch" false false)
  (bind _asbp_ball (Utilities|Casting|CastToBP_Ball OtherActor))
  (Default|AdjustBallSpeed _asbp_ball 0.0)
  (Audio|SpawnSoundAttached "/Game/Assets/Sounds/Pinball/Arcade_GameStart.Arcade_GameStart" (Variables|Default|GetBallHoleMesh) "None" "0, 0, 0" "0, 0, 0" "KeepRelativeOffset" false 1.0 1.0 0.0 0 0)
  (Development|PrintString "Black Hole" false false)
  (CallFunction|AddtoScore 5e+02)
  (Transformation|SetActorLocation _asbp_ball (Math|Vector|MakeVector (.x _returnvalue) (.y _returnvalue) (- (.z _returnvalue) 5e+01)) false false)
  (Utilities|FlowControl|Delay 0.5)
  (Audio|SpawnSoundAttached "/Game/Assets/Sounds/Pinball/transporter9.transporter9" (Variables|Default|GetBallHoleMesh) "None" "0, 0, 0" "0, 0, 0" "KeepRelativeOffset" false 1.0 1.0 0.0 0 0)
  (bind _scalealpha (Timeline|WarpBallAway PlayFromStart)
    (:Update
      (Transformation|SetActorScale3D _asbp_ball (Math|Vector|Lerp(Vector) (Transformation|GetActorScale3D _asbp_ball) "0, 0, 0" _scalealpha)))
    (:Finished
      (Actor|DestroyActor _asbp_ball)
      (bind _asbp_pinball_game_mode (Utilities|Casting|CastToBP_PinballGameMode (Game|GetGameMode)))
      (Default|SpawnBallatRandomKickerHole _asbp_pinball_game_mode))))

(fn ConstructionScript)

(fn AddtoScore
  (params (PointsToAdd :type Float%20%28single-precision%29))
  (bind _asbp_pinball_game_mode (Utilities|Casting|CastToBP_PinballGameMode (Game|GetGameMode)))
  (Default|AddScore _asbp_pinball_game_mode PointsToAdd))