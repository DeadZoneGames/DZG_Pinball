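; Pinball game mode that runs the game loop from main menu through ball spawning and loss to high-score entry.
; ResetGame restores class defaults, spawns a ball at the plunger and creates the HUD; DestroyBall respawns until balls run out.
; Score gains scale by a multiplier that lights matching table lights as it climbs, while kicker-hole locations are cached for random spawns.
; EndGame checks a lazily loaded, cached save to choose high-score entry or menu.
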(event Custom|SpawnBallAtPlunger
  (bind _outactors (Actor|GetAllActorsOfClass "/Game/Blueprints/BP_Plunger.BP_Plunger_C"))
  (Game|SpawnActorfromClass "/Game/Blueprints/BP_Ball.BP_Ball_C" (Math|Transform|MakeTransform (Default|GetBallSpawnLocation (Utilities|Array|Get(acopy) _outactors)) "0, 0, 0" "1,1,1") "Undefined" 0 0))

(event Custom|SetPlayerView
  (params (Camera :type Camera%20Actor%20Object%20Reference))
  (Game|Player|SetViewTargetwithBlend (Game|GetPlayerController 0) Camera 0.0 "VTBlend_Linear" 0.0 false))

(event Custom|EndGame
  (bind _currentsaveobject (CallFunction|GetSaveGameData))
  (if (<= (Utilities|Array|Length (Variables|/Game/GamePlay/BP_HighScoreSave.BP_HighScoreSave_C|GetSaveStruct _currentsaveobject)) 3)
    (CallFunction|CreateHighScoreList :!label _label)
    (else
      (bind _lowestscorestruct (Default|DetermineLowestScoreValue _currentsaveobject))
      (if (< (.score _lowestscorestruct) (Variables|Default|GetScore))
        (goto _label)
        (else
          (CallFunction|CreateMainMenu))))))

(event Custom|CreateHighScoreList
  (bind _returnvalue (Game|GetPlayerController 0))
  (bind _asbp_pinball_player_controller (Utilities|Casting|CastToBP_PinballPlayerController _returnvalue))
  (bind _returnvalue_2 (UserInterface|CreateWidget "/Game/UI/WBP_HighScoreEntry.WBP_HighScoreEntry_C" _asbp_pinball_player_controller))
  (UserInterface|Viewport|AddtoViewport _returnvalue_2 0)
  (Variables|/Script/Engine.PlayerController|SetbShowMouseCursor _asbp_pinball_player_controller true))

(event Custom|CreateMainMenu
  (bind _returnvalue (Game|GetPlayerController 0))
  (bind _asbp_pinball_player_controller (Utilities|Casting|CastToBP_PinballPlayerController _returnvalue))
  (CallFunction|GetSaveGameData)
  (bind _returnvalue_2 (UserInterface|CreateWidget "/Game/UI/WBP_MainMenu.WBP_MainMenu_C" _asbp_pinball_player_controller))
  (UserInterface|Viewport|AddtoViewport _returnvalue_2 0)
  (Input|SetInputModeUIOnly _asbp_pinball_player_controller 0 "DoNotLock")
  (Variables|/Script/Engine.PlayerController|SetbShowMouseCursor _asbp_pinball_player_controller true))

(event Custom|ResetGame
  (bind _returnvalue (Game|GetPlayerController 0))
  (bind (_score _multiplier _currentballnum _maxnumofballs _tiltcount) (Utilities|GetClassDefaults "BP_PinballGameMode_C"))
  (bind _asbp_pinball_player_controller (Utilities|Casting|CastToBP_PinballPlayerController _returnvalue))
  (Variables|Default|SetScore _score)
  (Variables|Default|SetMultiplier _multiplier)
  (Variables|Default|SetCurrentBallNum _currentballnum)
  (Variables|Default|SetMaxNumOfBalls _maxnumofballs)
  (Variables|Default|SetTiltCount _tiltcount)
  (CallFunction|SpawnBallatPlunger)
  (Default|CreatePlayerHUD _asbp_pinball_player_controller)
  (Variables|/Script/Engine.PlayerController|SetbShowMouseCursor _asbp_pinball_player_controller false)
  (Default|CallOnGameReset))

(event Custom|DetectKickerBallHoles
  (Utilities|Array|Clear (Variables|Default|GetKickerBallHoleLocations))
  (bind _outactors (Actor|GetAllActorsOfClass "/Game/Blueprints/BP_BallHoleKicker.BP_BallHoleKicker_C"))
  (for _array_element _outactors
    (Utilities|Array|Add (Variables|Default|GetKickerBallHoleLocations) (Transformation|GetActorLocation _array_element)))
  (Variables|Default|SetNumOfKickerBallHoleLocations (Utilities|Array|Length (Variables|Default|GetKickerBallHoleLocations))))

(event Custom|SpawnBallAtRandomKickerHole
  (bind _returnvalue (Transformation|GetActorLocation))
  (bind _numofkickerballholelocations (Variables|Default|GetNumOfKickerBallHoleLocations))
  (if (> _numofkickerballholelocations 0)
    (Game|SpawnActorfromClass "/Game/Blueprints/BP_Ball.BP_Ball_C" (Math|Transform|MakeTransform (Utilities|Array|Get(acopy) (Variables|Default|GetKickerBallHoleLocations) (Math|Random|RandomInteger _numofkickerballholelocations)) "0, 0, 0" "1,1,1") "Undefined" 0 0)
    (Transformation|SetActorLocation (Math|Vector|MakeVector (.x _returnvalue) (+ (.y _returnvalue) 5e+01) (+ (.z _returnvalue) 5e+01)) false false)))

(event Custom|DestroyBall
  (params (Ball :type BP%20Ball%20Object%20Reference))
  (Actor|DestroyActor Ball)
  (if (<= (+ (Variables|Default|GetCurrentBallNum) 1) (Variables|Default|GetMaxNumOfBalls))
    (Variables|Default|SetCurrentBallNum (+ (Variables|Default|GetCurrentBallNum) 1))
    (CallFunction|SpawnBallatPlunger)
    (else
      (CallFunction|EndGame))))

(event EventBeginPlay
  (CallFunction|DetectKickerBallHoles)
  (CallFunction|CreateMainMenu)
  (Audio|PlaySound2D "/Game/Assets/Sounds/8BitActionGameLoops/Loop_2_Cue.Loop_2_Cue" 0.1 1.0 0.0 0 0))

(fn ConstructionScript)

(fn AddScore
  (params (PointsToAdd :type Float%20%28single-precision%29))
  (bind _output_get (Variables|Default|SetScore (+ (* (Variables|Default|GetMultiplier) PointsToAdd) (Variables|Default|GetScore))))
  (return _output_get))

(fn GetSaveGameData
  (bind _currentsaveobject (Variables|Default|GetCurrentSaveObject)
    (:then
      (return _currentsaveobject))
    (:else
      (bind _returnvalue (SaveGame|DoesSaveGameExist (Variables|Default|GetHighScoreSaveName)))
      (if _returnvalue
        (bind _returnvalue_2 (SaveGame|LoadGamefromSlot (Variables|Default|GetHighScoreSaveName)))
        (bind _asbp_high_score_save (Utilities|Casting|CastToBP_HighScoreSave _returnvalue_2)
          (:then
            (Default|SortSaveData _asbp_high_score_save)
            (bind _output_get (Variables|Default|SetCurrentSaveObject _asbp_high_score_save))
            (return _output_get))
          (:CastFailed
            (return 0)))
        (else
          (bind _returnvalue_3 (SaveGame|CreateSaveGameObject "/Game/GamePlay/BP_HighScoreSave.BP_HighScoreSave_C"))
          (bind _output_get_2 (Variables|Default|SetCurrentSaveObject _returnvalue_3))
          (return _output_get_2))))))

(fn IncreaseMultiplier
  (bind _multiplier (Variables|Default|GetMultiplier))
  (if (< _multiplier 6)
    (bind _result (Math|Integer|IncrementInt _multiplier)
      (:%20%20
        (switch int _result
          (:2
            (bind _outactors (Actor|GetAllActorsOfClass "/Game/Blueprints/BP_TableLight_2X.BP_TableLight_2X_C"))
            (for _array_element _outactors
              (Rendering|Components|Light|SetIntensity (Variables|/Game/Blueprints/BP_TableLight.BP_TableLight_C|GetSpotLight _array_element) 1e+06)
              (Audio|PlaySound2D "/Game/Assets/Sounds/Other/arcade_game_level_up_tone_Cue.arcade_game_level_up_tone_Cue" 1.0 1.0 0.0 0 0)))
          (:3
            (bind _outactors_2 (Actor|GetAllActorsOfClass "/Game/Blueprints/BP_TableLight_3X.BP_TableLight_3X_C"))
            (for _array_element_2 _outactors_2
              (Rendering|Components|Light|SetIntensity (Variables|/Game/Blueprints/BP_TableLight.BP_TableLight_C|GetSpotLight _array_element_2) 1e+06)
              (Audio|PlaySound2D "/Game/Assets/Sounds/Other/arcade_game_level_up_tone_Cue.arcade_game_level_up_tone_Cue" 1.0 1.0 0.0 0 0)))
          (:4
            (bind _outactors_3 (Actor|GetAllActorsOfClass "/Game/Blueprints/BP_TableLight_4X.BP_TableLight_4X_C"))
            (for _array_element_3 _outactors_3
              (Rendering|Components|Light|SetIntensity (Variables|/Game/Blueprints/BP_TableLight.BP_TableLight_C|GetSpotLight _array_element_3) 1e+06)
              (Audio|PlaySound2D "/Game/Assets/Sounds/Other/arcade_game_level_up_tone_Cue.arcade_game_level_up_tone_Cue" 1.0 1.0 0.0 0 0)))
          (:5
            (Math|Integer|IncrementInt (Variables|Default|GetMultiplier)
              (:%20%20
                (bind _outactors_4 (Actor|GetAllActorsOfClass "/Game/Blueprints/BP_TableLight_6X.BP_TableLight_6X_C"))
                (for _array_element_4 _outactors_4
                  (Rendering|Components|Light|SetIntensity (Variables|/Game/Blueprints/BP_TableLight.BP_TableLight_C|GetSpotLight _array_element_4) 1e+06)
                  (Audio|PlaySound2D "/Game/Assets/Sounds/Other/arcade_game_level_up_tone_Cue.arcade_game_level_up_tone_Cue" 1.0 1.0 0.0 0 0))))))))))