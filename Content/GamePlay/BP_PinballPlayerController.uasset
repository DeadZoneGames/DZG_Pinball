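; Player controller for the pinball game that routes input to the table's flippers, plunger and ball hole launchers, and creates the HUD.
; On BeginPlay it caches those actors, sorting flippers by side; flipper and plunger inputs also rotate and charge the launchers.
; Tilt uses a limited game-mode count to impulse every ball and shake the camera directionally.
; Escape or Pause opens a reused in-game menu and pauses the game.
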(event Custom|DetectFlippers
  (bind _outactors (Actor|GetAllActorsOfClass "/Game/Blueprints/BP_Flipper.BP_Flipper_C"))
  (for _array_element _outactors
    (switch Utilities|FlowControl|Switch|SwitchonFlipType (Variables|/Game/Blueprints/BP_Flipper.BP_Flipper_C|GetFlipType _array_element)
      (:NewEnumerator0
        (Utilities|Array|Add (Variables|Default|GetRightFlippers) _array_element))
      (:NewEnumerator1
        (Utilities|Array|Add (Variables|Default|GetLeftFlippers) _array_element)))))

(event Custom|DetectPlunger
  (bind _outactors (Actor|GetAllActorsOfClass "/Game/Blueprints/BP_Plunger.BP_Plunger_C"))
  (Variables|Default|SetPlunger (Utilities|Array|Get(acopy) _outactors)))

(event Custom|CreatePlayerHUD
  (Viewport|RemoveAllWidgets)
  (bind _returnvalue (UserInterface|CreateWidget "/Game/UI/WBP_PinballHUD.WBP_PinballHUD_C"))
  (UserInterface|Viewport|AddtoViewport _returnvalue 0))

(event Custom|DetectBallLaunchers
  (bind _outactors (Actor|GetAllActorsOfClass "/Game/Blueprints/BP_BallHoleLauncher.BP_BallHoleLauncher_C"))
  (Variables|Default|SetBallHoleLaunchers _outactors))

(event EventBeginPlay
  (CallFunction|DetectFlippers)
  (CallFunction|DetectPlunger)
  (CallFunction|DetectBallLaunchers))

(event Input|ActionEvents|InputActionLeftFlipper
  (params (Key :type Key%20Structure :default "None"))
  (bind _leftflippers (Variables|Default|GetLeftFlippers))
  (:Pressed
    (for _array_element _leftflippers
      (Default|Flip _array_element))
    (for _array_element_2 (Variables|Default|GetBallHoleLaunchers)
      (Default|RotateLeft _array_element_2)))
  (:Released
    (for _array_element_3 _leftflippers
      (Default|Flop _array_element_3))
    (for _array_element_4 (Variables|Default|GetBallHoleLaunchers)
      (Default|StopRotation _array_element_4))))

(event Input|ActionEvents|InputActionRightFlipper
  (params (Key :type Key%20Structure :default "None"))
  (bind _rightflippers (Variables|Default|GetRightFlippers))
  (:Pressed
    (for _array_element _rightflippers
      (Default|Flip _array_element))
    (for _array_element_2 (Variables|Default|GetBallHoleLaunchers)
      (Default|RotateRight _array_element_2)))
  (:Released
    (for _array_element_3 _rightflippers
      (Default|Flop _array_element_3))
    (for _array_element_4 (Variables|Default|GetBallHoleLaunchers)
      (Default|StopRotation _array_element_4))))

(event Input|ActionEvents|InputActionPlunger
  (params (Key :type Key%20Structure :default "None"))
  (bind _plunger (Variables|Default|GetPlunger))
  (bind _ballholelaunchers (Variables|Default|GetBallHoleLaunchers))
  (:Pressed
    (Default|ChargePlunger _plunger)
    (for _array_element _ballholelaunchers
      (Default|ChargeLauncher _array_element)))
  (:Released
    (Default|StopCharge _plunger)
    (for _array_element_2 _ballholelaunchers
      (Default|StopCharge _array_element_2))))

(event Input|ActionEvents|InputActionLeftTilt
  (params (Key :type Key%20Structure :default "None"))
  (:Pressed
    (CallFunction|Tilt "NewEnumerator0")))

(event Input|ActionEvents|InputActionRightTilt
  (params (Key :type Key%20Structure :default "None"))
  (:Pressed
    (CallFunction|Tilt "NewEnumerator1")))

(event Input|ActionEvents|InputActionPause
  (params (Key :type Key%20Structure :default "None"))
  (bind _returnvalue (Game|GetPlayerController 0))
  (:Pressed
    (Utilities|IsValid (Variables|Default|GetInGameMenuRef)
      (:Is%20Valid
        _)
      (:Is%20Not%20Valid
        (bind _returnvalue_2 (UserInterface|CreateWidget "/Game/UI/WBP_InGameMenu.WBP_InGameMenu_C" _returnvalue))
        (Variables|Default|SetInGameMenuRef _returnvalue_2)))
    (UserInterface|Viewport|AddtoViewport (Variables|Default|GetInGameMenuRef) 0)
    (Input|SetInputModeUIOnly _returnvalue 0 "DoNotLock")
    (Variables|Default|SetbShowMouseCursor true)
    (Game|SetGamePaused true)))

(event Input|KeyboardEvents|Escape
  (params (Key :type Key%20Structure :default "None"))
  (bind _returnvalue (Game|GetPlayerController 0))
  (:Pressed
    (Utilities|IsValid (Variables|Default|GetInGameMenuRef)
      (:Is%20Valid
        _)
      (:Is%20Not%20Valid
        (bind _returnvalue_2 (UserInterface|CreateWidget "/Game/UI/WBP_InGameMenu.WBP_InGameMenu_C" _returnvalue))
        (Variables|Default|SetInGameMenuRef _returnvalue_2)))
    (UserInterface|Viewport|AddtoViewport (Variables|Default|GetInGameMenuRef) 0)
    (Input|SetInputModeUIOnly _returnvalue 0 "DoNotLock")
    (Variables|Default|SetbShowMouseCursor true)
    (Game|SetGamePaused true)))

(fn ConstructionScript)

(fn Tilt
  (params (TiltDirection :type FlipType%20Enum :default "NewEnumerator0"))
  (bind _returnvalue (Game|GetPlayerCameraManager 0))
  (bind _returnvalue_2 (Camera|GetCameraRotation _returnvalue))
  (if (> (Variables|/Game/GamePlay/BP_PinballGameMode.BP_PinballGameMode_C|GetTiltCount (.AsBP%20Pinball%20Game%20Mode (Utilities|Casting|CastToBP_PinballGameMode (Game|GetGameMode)))) 0)
    (bind _outactors (Actor|GetAllActorsOfClass "/Game/Blueprints/BP_Ball.BP_Ball_C"))
    (if (>= (Utilities|Array|Length _outactors) 1)
      (for _array_element _outactors
        (Physics|AddImpulse (Variables|/Game/Blueprints/BP_Ball.BP_Ball_C|GetBall _array_element) (Utilities|Select :Index TiltDirection :NewEnumerator0 "-500.000000,0.000000,0.000000" :NewEnumerator1 "500.000000, 0, 0") "None" true)
        (Class|PlayerController|ClientPlayCameraShake "/Game/GamePlay/BP_TiltShake.BP_TiltShake_C" 1.0 "UserDefined" (Utilities|Select :Index TiltDirection :NewEnumerator0 _returnvalue_2 :NewEnumerator1 (Math|Rotator|CombineRotators _returnvalue_2 "0,180.000000, 0"))))
      (Math|Integer|DecrementInt (Variables|/Game/GamePlay/BP_PinballGameMode.BP_PinballGameMode_C|GetTiltCount (.AsBP%20Pinball%20Game%20Mode (Utilities|Casting|CastToBP_PinballGameMode (Game|GetGameMode))))))))